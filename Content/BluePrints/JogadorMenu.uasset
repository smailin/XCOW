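; JogadorMenu is a player Blueprint, apparently for the menu, that shows the mouse cursor and turns the player to aim at it.
; BeginPlay enables the cursor, and Tick calls MirarComMouse.
; When UsarMouse is set, that function traces under the cursor on the Camera channel and interpolates control rotation from the pawn's rotation toward the hit point.
; Crosshair cursor, HUD widget and move-input nodes are left unconnected.
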(event EventBeginPlay
  ;[1 1 1] Coisas que iniciam com o jogador
  (Utilities|FlowControl|Sequence
    (:then_0
      (Variables|/Script/Engine.PlayerController|SetbShowMouseCursor (Game|GetPlayerController 0) true))))

(event EventTick
  (params (DeltaSeconds :type Float%20%28single-precision%29))
  ;[1 1 1] Coisas que iniciam com o jogador
  (CallFunction|MirarComMouse))

(fn ConstructionScript)

(fn MirarComMouse
  (bind _returnvalue (Game|GetPlayerController 0))
  (bind _returnvalue_2 (Pawn|GetControlledPawn _returnvalue))
  (if (Variables|Default|GetUsar%20mouse)
    (Pawn|SetControlRotation (Game|GetPlayerController 0) (Math|Interpolation|RInterpTo (Transformation|GetActorRotation _returnvalue_2) (Math|Rotator|FindLookatRotation (Transformation|GetActorLocation _returnvalue_2) (.Location (Collision|BreakHitResult (.HitResult (Game|Player|GetHitResultUnderCursorbyChannel _returnvalue "TraceTypeQuery2" true))))) (Utilities|Time|GetWorldDeltaSeconds) 6e+01))
    (return)))