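; Barrier actor that the player raises with the Formar Barreira input by spending skulls (Caveiras), and that aliens can knock down.
; If skulls reach CaveirasNecessarias, it deducts a hardcoded 5, plays Death's casting animation and lifts Cube and Box via MoveComponentTo, with collision off until a delay ends.
; Alien_01 overlaps on Box drain Health; at zero the barrier sinks, Health resets and it can be raised again.
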(event OnComponentBeginOverlap(Box)
  (params (OverlappedComponent :type Primitive%20Component%20Object%20Reference) (OtherActor :type Actor%20Object%20Reference) (OtherComp :type Primitive%20Component%20Object%20Reference) (OtherBodyIndex :type Integer) (bFromSweep :type Boolean) (SweepResult :type Hit%20Result%20Structure%20%28by%20ref%29))
  (bind _cube (Variables|Default|GetCube))
  (bind _box (Variables|Default|GetBox))
  (bind _returnvalue (Transformation|GetRelativeTransform _cube))
  (bind _returnvalue_2 (Transformation|GetRelativeTransform _box))
  (Utilities|Casting|CastToAlien_01 OtherActor)
  (Variables|Default|Sethealth (- (Variables|Default|Gethealth) (Variables|Default|GetDano%20do%20tiro%20do%20alien)))
  (if (<= (Variables|Default|Gethealth) 0.0)
    (Variables|Default|SetFeita false)
    (Components|MoveComponentTo _cube (Math|Vector|MakeVector (.x (.location _returnvalue)) (.y (.location _returnvalue)) -1e+02) (.rotation _returnvalue) false true 2.0 false)
    (Components|MoveComponentTo _box (Math|Vector|MakeVector (.x (.location _returnvalue_2)) (.y (.location _returnvalue_2)) -1e+02) (.rotation _returnvalue_2) false true 1.0 false)
    (Variables|Default|Sethealth 1e+02)))

(event EventBeginPlay)

(event Collision|EventActorBeginOverlap
  (params (OtherActor :type Actor%20Object%20Reference)))

(event EventTick
  (params (DeltaSeconds :type Float%20%28single-precision%29)))

(event Input|ActionEvents|InputActionFormarBarreira
  (params (Key :type Key%20Structure))
  (bind _death (Variables|Default|GetDeath))
  (bind _cube (Variables|Default|GetCube))
  (bind _death_2 (Variables|Default|GetDeath))
  (bind _box (Variables|Default|GetBox))
  (bind _returnvalue (Transformation|GetRelativeTransform _cube))
  (bind _returnvalue_2 (Transformation|GetRelativeTransform _box))
  (:Pressed
    (bind _asjogador (Utilities|Casting|CastToJogador (Game|GetPlayerCharacter 0)))
    (if (>= (Variables|/Game/BluePrints/Jogador.Jogador_C|GetCaveiras _asjogador) (Variables|Default|GetCaveiras%20Necessarias))
      (if (not (Variables|Default|GetFeita))
        (Variables|/Game/BluePrints/Jogador.Jogador_C|SetCaveiras _asjogador (- (Variables|/Game/BluePrints/Jogador.Jogador_C|GetCaveiras _asjogador) 5.0))
        (Audio|PlaySound2D "/Game/SFX/Transmutação_Cue.Transmutação_Cue")
        (Transformation|SetRelativeRotation _death "0,110.000000, 0" false false)
        (Components|Animation|PlayAnimation _death "/Game/Animações/Death_Magic_Attack.Death_Magic_Attack" false)
        (Collision|SetCollisionEnabled (Variables|Default|GetCube) "NoCollision")
        (Collision|SetCollisionEnabled (Variables|Default|GetBox) "NoCollision")
        (Components|MoveComponentTo _cube (Math|Vector|MakeVector (.x (.location _returnvalue)) (.y (.location _returnvalue)) 1e+02) (.rotation _returnvalue) false true 1.0 false)
        (Variables|Default|SetFeita true)
        (Components|MoveComponentTo _box (Math|Vector|MakeVector (.x (.location _returnvalue_2)) (.y (.location _returnvalue_2)) 1e+02) (.rotation _returnvalue_2) false true 1.0 false)
        (Utilities|FlowControl|Delay 2.0)
        (Transformation|SetRelativeRotation _death_2 "0,7.000000, 0" false false)
        (Components|Animation|SetAnimation _death_2 "/Game/Animações/Death_Idle.Death_Idle")
        (Collision|SetCollisionEnabled (Variables|Default|GetCube) "QueryAndPhysics")
        (Collision|SetCollisionEnabled (Variables|Default|GetBox) "QueryAndPhysics")))))

(fn ConstructionScript)