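; Barn actor that stages an alien abduction, ending the player's game if aliens stay inside its trigger box.
; Box overlaps count Alien_01 actors, and Tick starts Abduzir when any are present: a siren plays and four legs descend one by one with mothership sounds.
; After a delay, remaining aliens trigger Cutscene, lifting the Barn and calling GameOver on Jogador.
; Otherwise the siren stops and the legs retract and hide.
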(event OnComponentBeginOverlap(Box)
  (params (OverlappedComponent :type Primitive%20Component%20Object%20Reference) (OtherActor :type Actor%20Object%20Reference) (OtherComp :type Primitive%20Component%20Object%20Reference) (OtherBodyIndex :type Integer) (bFromSweep :type Boolean) (SweepResult :type Hit%20Result%20Structure%20%28by%20ref%29))
  (Utilities|Casting|CastToAlien_01 OtherActor)
  (Variables|Default|Setquantos%20aliens (+ (Variables|Default|Getquantos%20aliens) 1.0)))

(event OnComponentEndOverlap(Box)
  (params (OverlappedComponent :type Primitive%20Component%20Object%20Reference) (OtherActor :type Actor%20Object%20Reference) (OtherComp :type Primitive%20Component%20Object%20Reference) (OtherBodyIndex :type Integer))
  (Utilities|Casting|CastToAlien_01 OtherActor)
  (Variables|Default|Setquantos%20aliens (- (Variables|Default|Getquantos%20aliens) 1.0)))

(event Custom|Abduzir
  (bind _perna01 (Variables|Default|GetPerna01))
  (bind _perna03 (Variables|Default|GetPerna03))
  (bind _perna02 (Variables|Default|GetPerna02))
  (bind _perna04 (Variables|Default|GetPerna04))
  (bind _returnvalue (Transformation|GetRelativeTransform _perna01))
  (bind _returnvalue_2 (Transformation|GetRelativeTransform _perna02))
  (bind _returnvalue_3 (Transformation|GetRelativeTransform _perna03))
  (bind _returnvalue_4 (Transformation|GetRelativeTransform _perna04))
  (Variables|Default|Setanimando true)
  (Audio|Components|Audio|Play (Variables|Default|GetSirene) 0.0)
  (Development|SetHiddeninGame (Variables|Default|GetPerna02) false false)
  (Components|MoveComponentTo _perna01 (Math|Vector|MakeVector (.x (.location _returnvalue)) (.y (.location _returnvalue)) 0.0) (.rotation _returnvalue) false false 1.0 false)
  (Audio|PlaySoundatLocation "/Game/SFX/NaveMae_Cue.NaveMae_Cue" (Transformation|GetWorldLocation _perna01))
  (Components|MoveComponentTo _perna02 (Math|Vector|MakeVector (.x (.location _returnvalue_2)) (.y (.location _returnvalue_2)) 0.0) (.rotation _returnvalue_2) false false 1.0 false)
  (Audio|PlaySoundatLocation "/Game/SFX/NaveMae_Cue.NaveMae_Cue" (Transformation|GetWorldLocation _perna02))
  (Components|MoveComponentTo _perna03 (Math|Vector|MakeVector (.x (.location _returnvalue_3)) (.y (.location _returnvalue_3)) 0.0) (.rotation _returnvalue_3) false false 1.0 false)
  (Audio|PlaySoundatLocation "/Game/SFX/NaveMae_Cue.NaveMae_Cue" (Transformation|GetWorldLocation _perna03))
  (Components|MoveComponentTo _perna04 (Math|Vector|MakeVector (.x (.location _returnvalue_4)) (.y (.location _returnvalue_4)) 0.0) (.rotation _returnvalue_4) false false 1.0 false)
  (Audio|PlaySoundatLocation "/Game/SFX/NaveMae_Cue.NaveMae_Cue" (Transformation|GetWorldLocation _perna04))
  (Utilities|FlowControl|Delay 13.0)
  (if (>= (Variables|Default|Getquantos%20aliens) 1.0)
    (CallFunction|Cutscene)
    (else
      (Audio|Components|Audio|Stop (Variables|Default|GetSirene))
      (CallFunction|RecolhaPernas))))

(event Custom|Cutscene
  (Variables|Default|SetAcabou true)
  (Components|MoveComponentTo (Variables|Default|GetBarn) "0.0,0.0,500.000000" "0, 0, 0" false false 7.0 false)
  (Variables|Default|Setanimando false)
  (bind _asjogador (Utilities|Casting|CastToJogador (Game|GetPlayerCharacter 0)))
  (Variables|/Game/BluePrints/Jogador.Jogador_C|SetGameOver _asjogador true)
  (Default|GameOver _asjogador))

(event Custom|Recolha%20pernas
  (bind _perna02 (Variables|Default|GetPerna02))
  (bind _perna03 (Variables|Default|GetPerna03))
  (bind _perna04 (Variables|Default|GetPerna04))
  (bind _perna01 (Variables|Default|GetPerna01))
  (bind _returnvalue (Transformation|GetRelativeTransform _perna02))
  (bind _returnvalue_2 (Transformation|GetRelativeTransform _perna03))
  (bind _returnvalue_3 (Transformation|GetRelativeTransform _perna04))
  (bind _returnvalue_4 (Transformation|GetRelativeTransform _perna01))
  (Variables|Default|Setrecolhendo true)
  (Components|MoveComponentTo _perna01 (Math|Vector|MakeVector (.x (.location _returnvalue_4)) (.y (.location _returnvalue_4)) 1e+03) (.rotation _returnvalue_4) false false 1.0 false)
  (Components|MoveComponentTo _perna02 (Math|Vector|MakeVector (.x (.location _returnvalue)) (.y (.location _returnvalue)) 1e+03) (.rotation _returnvalue) false false 1.0 false)
  (Components|MoveComponentTo _perna03 (Math|Vector|MakeVector (.x (.location _returnvalue_2)) (.y (.location _returnvalue_2)) 1e+03) (.rotation _returnvalue_2) false false 1.0 false)
  (Components|MoveComponentTo _perna04 (Math|Vector|MakeVector (.x (.location _returnvalue_3)) (.y (.location _returnvalue_3)) 1e+03) (.rotation _returnvalue_3) false false 1.0 false)
  (Development|SetHiddeninGame (Variables|Default|GetPerna02) true false)
  (Variables|Default|Setrecolhendo false)
  (Variables|Default|Setanimando false))

(event EventBeginPlay
  (Utilities|FlowControl|Sequence
    (:then_0
      (Variables|Default|SetAbduzindo false))
    (:then_1
      (Variables|Default|Setanimando false))
    (:then_2
      (Variables|Default|Setrecolhendo false))
    (:then_3
      (Variables|Default|Setquantos%20aliens 0.0))))

(event Collision|EventActorBeginOverlap
  (params (OtherActor :type Actor%20Object%20Reference)))

(event EventTick
  (params (DeltaSeconds :type Float%20%28single-precision%29))
  (if (not (Variables|Default|Getrecolhendo))
    (if (not (Variables|Default|GetAcabou))
      (if (>= (Variables|Default|Getquantos%20aliens) 1.0)
        (if (not (Variables|Default|Getanimando))
          (CallFunction|Abduzir))))))

(fn ConstructionScript)