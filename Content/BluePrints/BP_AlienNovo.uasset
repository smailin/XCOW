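; BP_AlienNovo is an AI-controlled alien that heads for a farm target and diverts toward the player when it sees them.
; Tick issues the farm move when both the seen and moving flags are clear.
; PawnSensing sightings of a Jogador pawn start a move to within a wide acceptance radius of it.
; A retriggerable five-second delay, restarted by sightings, then clears both flags so the farm move resumes.
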(event OnSeePawn(PawnSensing)
  (params (Pawn :type Pawn%20Object%20Reference))
  (Variables|Default|SetSeen_0 true)
  (bind _asjogador (Utilities|Casting|CastToJogador Pawn))
  (AI|AIMoveTo self "0, 0, 0" _asjogador 8e+02 false
    (:then
      (Utilities|FlowControl|RetriggerableDelay 5.0)
      (Variables|Default|SetSeen_0 false)
      (Variables|Default|SetMoving_0 false))))

(event Collision|EventActorBeginOverlap
  (params (OtherActor :type Actor%20Object%20Reference))
  (|CallParentFunction OtherActor))

(event EventTick
  (params (DeltaSeconds :type Float%20%28single-precision%29))
  (if (not (Variables|Default|GetSeen_0))
    (if (not (Variables|Default|GetMoving_0))
      (AI|AIMoveTo self "0, 0, 0" (Variables|Default|GetFarm_0) 5.0 false
        (:then
          (Variables|Default|SetMoving_0 true))
        (:OnSuccess
          (Variables|Default|SetMoving_0 false))))))

(fn ConstructionScript
  (|CallParentFunction))