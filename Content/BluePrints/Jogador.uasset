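; Player character for a top-down shooter: a farmer who fights aliens and carries cows to a drop-off.
; Aims by mouse-cursor trace or gamepad stick; a Tick gate drives cooldown-limited fire from a three-projectile shotgun or picked-up laser.
; Carrying a cow blocks firing, slows movement and swaps the anim class; delivery restores health and raises VACOMETRO.
; A full meter wins; an empty meter or zero health loses, both returning to the menu.
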(event OnComponentEndOverlap(Box)
  (params (OverlappedComponent :type Primitive%20Component%20Object%20Reference) (OtherActor :type Actor%20Object%20Reference) (OtherComp :type Primitive%20Component%20Object%20Reference) (OtherBodyIndex :type Integer))
  ;[1 1 1] Levar Dano
  (bind _asprojetil_alien (Utilities|Casting|CastToProjetilAlien OtherActor))
  (Camera|PlayWorldCameraShake "/Game/BluePrints/CameraDano1.CameraDano1_C" (Transformation|GetWorldLocation (Variables|Default|GetCamera%20do%20Personagem)) 0.0 5e+02)
  (Variables|Default|SetHEALTH (- (Variables|Default|GetHEALTH) (Variables|Default|GetDano%20recebido)))
  (Actor|DestroyActor _asprojetil_alien)
  (Audio|PlaySound2D "/Game/SFX/Dano_fazendeiro/Dano_fazendeiro.Dano_fazendeiro")
  (if (<= (Variables|Default|GetHEALTH) 0.0)
    (CallFunction|GameOver)))

(event OnComponentBeginOverlap(Box)
  (params (OverlappedComponent :type Primitive%20Component%20Object%20Reference) (OtherActor :type Actor%20Object%20Reference) (OtherComp :type Primitive%20Component%20Object%20Reference) (OtherBodyIndex :type Integer) (bFromSweep :type Boolean) (SweepResult :type Hit%20Result%20Structure%20%28by%20ref%29))
  ;[1 1 1] Pegar Arma do Chão
  (bind _aslazer_gun_item (Utilities|Casting|CastToLazerGun_Item OtherActor))
  (Variables|Default|SetPegou%20Arma%20nova true)
  (CallFunction|PegarArma)
  (Audio|PlaySound2D "/Game/SFX/Pegar_Arma.Pegar_Arma" 0.0)
  (Actor|DestroyActor _aslazer_gun_item)
  (CallFunction|Tougle))

(event OnComponentBeginOverlap(CapsuleComponent)
  (params (OverlappedComponent :type Primitive%20Component%20Object%20Reference) (OtherActor :type Actor%20Object%20Reference) (OtherComp :type Primitive%20Component%20Object%20Reference) (OtherBodyIndex :type Integer) (bFromSweep :type Boolean) (SweepResult :type Hit%20Result%20Structure%20%28by%20ref%29))
  ;[1 1 1] Entrega a Vaca
  (Utilities|Casting|CastToEntregaVacaBP OtherActor)
  (if (Variables|Default|GetTem%20Vaca)
    (Audio|PlaySound2D "/Game/SFX/outros/SFX_entregando_vaca.SFX_entregando_vaca")
    (Actor|DestroyActor (Variables|Default|GetVarVaca))
    (Variables|Default|SetTem%20Vaca false)
    (Variables|Default|SetNumeroVacas (+ (Variables|Default|GetNumeroVacas) 1.0))
    (Components|SkeletalMesh|SetAnimInstanceClass (Variables|Character|GetMesh) "/Game/Animações/Fazen_AnimBlueprint.Fazen_AnimBlueprint_C")
    (CallFunction|PegarArma)
    (Variables|/Script/Engine.CharacterMovementComponent|SetMaxWalkSpeed (Variables|Character|GetCharacterMovement) 7e+02)
    (Variables|Default|SetVACOMETRO (+ (Variables|Default|GetVACOMETRO) 1e+01))
    (Variables|Default|SetHEALTH (+ (Variables|Default|GetHEALTH) 5.0))
    (if (>= (Variables|Default|GetVACOMETRO) 1e+02)
      (Variables|Default|SetVenceu true)
      (Collision|SetCollisionEnabled (Variables|Collision|GetCapsuleComponent) "NoCollision")
      (Input|DisableInput 0)
      (Audio|Components|Audio|FadeOut (Variables|Default|GetMusic) 1.0 0.0 :!class /Script/Engine.AudioComponent)
      (Audio|PlaySound2D "/Game/Musicas/jam_vitória_bateria.jam_vitória_bateria" 0.1)
      (Utilities|FlowControl|Delay 8.0)
      (Game|OpenLevel(byName) "MapaMenu")
      (Actor|DestroyActor))))

(event Custom|Pull%20Trigger
  ;[1 1 1] tiros
  (Utilities|FlowControl|DoOnce false
    (:Completed
      (CallFunction|Fire)
      (Utilities|Time|SetTimerbyFunctionName 0 "" (/ 1.0 (Variables|Default|GetColdown%20Rifle))))))

(event Custom|Desligar%20mouse
  (bind _returnvalue (Game|GetPlayerController 0))
  (Variables|/Script/Engine.PlayerController|SetbShowMouseCursor _returnvalue false)
  (Variables|/Script/Engine.PlayerController|SetbEnableMouseOverEvents _returnvalue false)
  (Variables|/Script/Engine.PlayerController|SetbEnableClickEvents _returnvalue false))

(event Custom|Game%20Over
  ;[1 1 1] Game Over
  (Variables|Default|SetGameOver true)
  (if (Variables|Default|GetTem%20Vaca)
    (Actor|DestroyActor (Variables|Default|GetVarVaca)))
  (Collision|SetCollisionEnabled (Variables|Default|GetBox) "NoCollision")
  (Input|DisableInput 0)
  (Components|Animation|PlayAnimation (Variables|Character|GetMesh) "/Game/Animações/Fazen_Dying.Fazen_Dying" false)
  (Audio|PlaySound2D "/Game/SFX/Fazen_Dying.Fazen_Dying")
  (Audio|Components|Audio|FadeOut (Variables|Default|GetMusic) 1.0 0.0 :!class /Script/Engine.AudioComponent)
  (Audio|PlaySound2D "/Game/Musicas/jam_derrota.jam_derrota" 0.1)
  (Utilities|FlowControl|Delay 8.0)
  (Game|OpenLevel(byName) "MapaMenu")
  (Actor|DestroyActor))

(event Custom|Release%20Trigger
  ;[1 1 1] tiros
  (Utilities|Time|ClearTimerbyFunctionName 0 "")
  (Utilities|FlowControl|DoOnce false) ; enters at Reset
)

(event Custom|Pegar%20Arma
  (bind _mesh (Variables|Character|GetMesh))
  (bind _mesh_2 (Variables|Character|GetMesh))
  (bind _pegou_arma_nova (Variables|Default|GetPegou%20Arma%20nova))
  ;[1 1 1] Verifica a arma e coloca a corrata na mão
  (if (Variables|Default|GetQual%20arma)
    (Actor|DestroyActor (Variables|Default|GetVarArma2) :!label _label)
    (if _pegou_arma_nova
      (Audio|PlaySound2D "/Game/SFX/outros/SFX_pega_espingarda_01.SFX_pega_espingarda_01"))
    (bind _returnvalue (Game|SpawnActorfromClass "/Game/BluePrints/Arma.Arma_C" (Transformation|GetRelativeTransform _mesh) "AlwaysSpawn" 0 0))
    (bind _output_get (Variables|Default|SetVarArma _returnvalue))
    (Transformation|AttachComponentToComponent _output_get _mesh "GunSocket" "SnapToTarget" "KeepRelative" "KeepRelative" true)
    (elif _pegou_arma_nova
      (Actor|DestroyActor (Variables|Default|GetVarArma))
      (bind _returnvalue_2 (Game|SpawnActorfromClass "/Game/BluePrints/Arma2.Arma2_C" (Transformation|GetRelativeTransform _mesh_2) "AlwaysSpawn" 0 0))
      (bind _output_get_2 (Variables|Default|SetVarArma2 _returnvalue_2))
      (Transformation|AttachComponentToComponent _output_get_2 _mesh_2 "GunSocket" "SnapToTarget" "KeepRelative" "KeepRelative" false)
      (else
        (goto _label)))))

(event Custom|Pegar%20Vaca
  (bind _mesh (Variables|Character|GetMesh))
  ;[1 1 1] Pega a Vaca
  (Actor|DestroyActor (Variables|Default|GetVarArma))
  (Audio|PlaySound2D "/Game/SFX/PegandoAVaca_Cue.PegandoAVaca_Cue")
  (if (not (Variables|Default|GetTem%20Vaca))
    (bind _returnvalue (Game|SpawnActorfromClass "/Game/BluePrints/Vaca_ItenBlueprint.Vaca_ItenBlueprint_C" (Transformation|GetWorldTransform _mesh) "AlwaysSpawn" 0 0))
    (bind _output_get (Variables|Default|SetVarVaca _returnvalue))
    (Transformation|AttachComponentToComponent _output_get _mesh "CowSocket" "SnapToTarget" "KeepRelative" "KeepRelative" true)
    (Variables|Default|SetTem%20Vaca true)
    (Components|SkeletalMesh|SetAnimInstanceClass (Variables|Character|GetMesh) "/Game/Animações/CarryCowBlendSpace.CarryCowBlendSpace_C")
    (Variables|/Script/Engine.CharacterMovementComponent|SetMaxWalkSpeed (Variables|Character|GetCharacterMovement) 5e+02)))

(event Custom|Ligar%20Mouse
  (bind _returnvalue (Game|GetPlayerController 0))
  (Variables|/Script/Engine.PlayerController|SetbShowMouseCursor _returnvalue true)
  (Variables|/Script/Engine.PlayerController|SetbEnableMouseOverEvents _returnvalue true)
  (Variables|/Script/Engine.PlayerController|SetbEnableClickEvents _returnvalue true))

(event Custom|Tougle
  ;[1 1 1] Verifica a arma e coloca a corrata na mão
  (if (Variables|Default|GetQual%20arma)
    (Variables|Default|SetQual%20arma false)
    (CallFunction|PegarArma)
    (else
      (Variables|Default|SetQual%20arma true)
      (CallFunction|PegarArma))))

(event Custom|Fire
  (bind _guntemp (Variables|Default|GetGunTemp))
  (bind _returnvalue (Transformation|GetWorldTransform _guntemp))
  ;[1 1 1] tiros
  (if (not (Variables|Default|GetTem%20Vaca))
    (if (Variables|Default|GetQual%20arma)
      (if (Variables|Default|GetColdDown) :!label _label
        (Audio|PlaySound2D "/Game/SFX/Tiro_Espingarda_Audio.Tiro_Espingarda_Audio")
        (Game|SpawnActorfromClass "/Game/BluePrints/ProjetilDoHeroi.ProjetilDoHeroi_C" _returnvalue "Undefined" 0 0)
        (Game|SpawnActorfromClass "/Game/BluePrints/ProjetilDoHeroi.ProjetilDoHeroi_C" (Transformation|GetWorldTransform (Variables|Default|GetGunTemp2)) "Undefined" 0 0)
        (Game|SpawnActorfromClass "/Game/BluePrints/ProjetilDoHeroi.ProjetilDoHeroi_C" (Transformation|GetWorldTransform (Variables|Default|GetGunTemp3)) "Undefined" 0 0)
        (Audio|PlaySound2D 0)
        (Variables|Default|SetColdDown false)
        (Utilities|FlowControl|Delay (Variables|Default|GetColdown%20Rifle))
        (Variables|Default|SetColdDown true))
      (elif (Variables|Default|GetPegou%20Arma%20nova)
        (if (Variables|Default|GetColdDown)
          (Game|SpawnActorfromClass "/Game/BluePrints/ProjetilDoHeroi_2.ProjetilDoHeroi_2_C" _returnvalue "Undefined" 0 0)
          (Audio|PlaySound2D "/Game/SFX/Tiro_laser_Audio.Tiro_laser_Audio")
          (Variables|Default|SetColdDown false)
          (Utilities|FlowControl|Delay (Variables|Default|GetColdown%20Laser))
          (Variables|Default|SetColdDown true))
        (else
          (goto _label))))))

(event EventBeginPlay
  (bind _returnvalue (Game|GetPlayerController 0))
  ;[1 1 1] Coisas que iniciam com o jogador
  (Utilities|FlowControl|Sequence
    (:then_0
      (Variables|/Script/Engine.PlayerController|SetbShowMouseCursor _returnvalue true)
      (Input|SetIgnoreMoveInput _returnvalue false))
    (:then_1
      (CallFunction|PegarArma))
    (:then_2
      (bind _returnvalue_2 (UserInterface|CreateWidget "/Game/HUD_GAMEWIDGET.HUD_GAMEWIDGET_C"))
      (UserInterface|Viewport|AddtoViewport _returnvalue_2 0))
    (:then_3
      (Variables|Default|SetVACOMETRO 5e+01))
    (:then_4
      (Class|PlayerController|SetMouseCursorWidget (Game|GetPlayerController 0) "None"))
    (:then_5
      (bind _asmodo_de_jogo (Utilities|Casting|CastToModoDeJogo (Game|GetGameMode)))
      (bind _output_get (Variables|Default|SetGamemode _asmodo_de_jogo))
      (Variables|/Game/ModoDeJogo.ModoDeJogo_C|SetPlayerSpawnTransform _output_get (Transformation|GetActorTransform)))
    (:then_6
      (Variables|Default|SetMorto false))
    (:then_7
      (Variables|Default|SetHEALTH 1e+02))
    (:then_8
      (Collision|SetCollisionEnabled (Variables|Collision|GetCapsuleComponent) "QueryAndPhysics")
      (Variables|Default|SetGameOver false))
    (:then_9
      (if (Variables|Default|GetUsar%20controle?)
        (CallFunction|DesligarMouse)
        (else
          (CallFunction|LigarMouse))))))

(event EventTick
  (params (DeltaSeconds :type Float%20%28single-precision%29))
  (bind _guntemp (Variables|Default|GetGunTemp))
  (bind _crosshair_controle (Variables|Default|GetCrossHair%20Controle))
  (bind _returnvalue (Transformation|GetWorldTransform _guntemp))
  (if (Variables|Default|GetUsar%20controle?)
    (Rendering|SetVisibility _crosshair_controle true false)
    (else
      (Rendering|SetVisibility _crosshair_controle false false)
      (CallFunction|MirarComMouse)))
  (if (not (<= (Variables|Default|GetVACOMETRO) 0.0))
    ;[1 1 1] tiros
    (Utilities|FlowControl|Gate true
      (:Exit
        (if (not (Variables|Default|GetTem%20Vaca))
          (if (Variables|Default|GetQual%20arma)
            (if (Variables|Default|GetColdDown) :!label _label
              (Audio|PlaySound2D "/Game/SFX/Tiro_Espingarda_Audio.Tiro_Espingarda_Audio")
              (Game|SpawnActorfromClass "/Game/BluePrints/ProjetilDoHeroi.ProjetilDoHeroi_C" _returnvalue "Undefined" 0 0)
              (Game|SpawnActorfromClass "/Game/BluePrints/ProjetilDoHeroi.ProjetilDoHeroi_C" (Transformation|GetWorldTransform (Variables|Default|GetGunTemp2)) "Undefined" 0 0)
              (Game|SpawnActorfromClass "/Game/BluePrints/ProjetilDoHeroi.ProjetilDoHeroi_C" (Transformation|GetWorldTransform (Variables|Default|GetGunTemp3)) "Undefined" 0 0)
              (Audio|PlaySound2D 0)
              (Variables|Default|SetColdDown false)
              (Utilities|FlowControl|Delay (Variables|Default|GetColdown%20Rifle))
              (Variables|Default|SetColdDown true))
            (elif (Variables|Default|GetPegou%20Arma%20nova)
              (if (Variables|Default|GetColdDown)
                (Game|SpawnActorfromClass "/Game/BluePrints/ProjetilDoHeroi_2.ProjetilDoHeroi_2_C" _returnvalue "Undefined" 0 0)
                (Audio|PlaySound2D "/Game/SFX/Tiro_laser_Audio.Tiro_laser_Audio")
                (Variables|Default|SetColdDown false)
                (Utilities|FlowControl|Delay (Variables|Default|GetColdown%20Laser))
                (Variables|Default|SetColdDown true))
              (else
                (goto _label)))))))
    (else
      (Utilities|FlowControl|DoOnce false
        (:Completed
          (CallFunction|GameOver))))))

(event Input|ActionEvents|InputActionAtirar
  (params (Key :type Key%20Structure))
  (bind _guntemp (Variables|Default|GetGunTemp))
  (bind _returnvalue (Transformation|GetWorldTransform _guntemp))
  ;[1 1 1] tiros
  (:Pressed
    (Utilities|FlowControl|Gate true) ; enters at Open
  )
  (:Released
    (Utilities|FlowControl|Gate true) ; enters at Close
  ))

(event Input|ActionEvents|InputActionTrocar
  (params (Key :type Key%20Structure))
  ;[1 1 1] Verifica a arma e coloca a corrata na mão
  (:Pressed
    (CallFunction|Tougle)))

(event Input|ActionEvents|InputActionAtirar
  (params (Key :type Key%20Structure))
  ;[1 1 1] Atirar
  (:Pressed
    (CallFunction|PullTrigger))
  (:Released
    (CallFunction|ReleaseTrigger)))

(event Input|AxisEvents|InputAxisMoveRight
  (params (AxisValue :type Float%20%28single-precision%29))
  ;[1 1 1] Movimento
  (Pawn|Input|AddMovementInput "0,1.000000, 0" AxisValue false))

(event Input|AxisEvents|InputAxisLookRight
  (params (AxisValue :type Float%20%28single-precision%29))
  ;[1 1 1] Rotação
  (if (> (Math|Vector|VectorLength (Math|Vector|MakeVector (stale Input|AxisEvents|InputAxisLookUp AxisValue) AxisValue 0.0)) 0.25)
    (Pawn|SetControlRotation (Pawn|GetController) (Math|Conversions|RotationFromXVector (Math|Vector|MakeVector (stale Input|AxisEvents|InputAxisLookUp AxisValue) AxisValue 0.0)))))

(event Input|AxisEvents|InputAxisMoveUp
  (params (AxisValue :type Float%20%28single-precision%29))
  ;[1 1 1] Movimento
  (Pawn|Input|AddMovementInput "1.000000, 0, 0" AxisValue false))

(event Input|AxisEvents|InputAxisLookUp
  (params (AxisValue :type Float%20%28single-precision%29))
  ;[1 1 1] Rotação
  (if (> (Math|Vector|VectorLength (Math|Vector|MakeVector AxisValue (stale Input|AxisEvents|InputAxisLookRight AxisValue) 0.0)) 0.25)
    (Pawn|SetControlRotation (Pawn|GetController) (Math|Conversions|RotationFromXVector (Math|Vector|MakeVector AxisValue (stale Input|AxisEvents|InputAxisLookRight AxisValue) 0.0)))))

(fn ConstructionScript)

(fn MirarComMouse
  (bind _returnvalue (Game|GetPlayerController 0))
  (bind _returnvalue_2 (Pawn|GetControlledPawn _returnvalue))
  (if (not (Variables|Default|GetUsar%20controle?))
    (Pawn|SetControlRotation (Game|GetPlayerController 0) (Math|Interpolation|RInterpTo (Transformation|GetActorRotation _returnvalue_2) (Math|Rotator|FindLookatRotation (Transformation|GetActorLocation _returnvalue_2) (.Location (Collision|BreakHitResult (.HitResult (Game|Player|GetHitResultUnderCursorbyChannel _returnvalue "TraceTypeQuery2" true))))) (Utilities|Time|GetWorldDeltaSeconds) 6e+01))
    (return)))