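; Alien enemy that marches to a fixed farm destination and attacks the player (Jogador) on sight.
; Tick drives the walk until PawnSensing spots a pawn, then it chases the player and fires ProjetilAlien from its gun.
; Capsule overlaps apply rifle or laser projectile damage.
; Death adds a skull to the player, plays an animation, sinks the mesh and drops a LazerGun_Item before destroying the actor.
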(event OnSeePawn(PawnSensing)
  (params (Pawn :type Pawn%20Object%20Reference))
  ;[1 0.269 0.3188] Ver Player
  (Variables|Default|SetSeen true)
  (if (not (Variables|Default|GetNa%20Fazenda))
    (bind _asjogador (Utilities|Casting|CastToJogador Pawn))
    (Variables|Default|SetJogador _asjogador)
    (AI|AIMoveTo self "0, 0, 0" _asjogador 5e+02 false
      (:then
        (CallFunction|Atacar _asjogador)
        (Utilities|FlowControl|RetriggerableDelay 1.0)
        (Variables|Default|SetSeen false)
        (Variables|Default|SetMoving false))
      (:OnSuccess
        (Variables|Default|SetClose%20Enough true))
      (:OnFail
        (Variables|Default|SetClose%20Enough false)))))

(event OnComponentBeginOverlap(CapsuleComponent)
  (params (OverlappedComponent :type Primitive%20Component%20Object%20Reference) (OtherActor :type Actor%20Object%20Reference) (OtherComp :type Primitive%20Component%20Object%20Reference) (OtherBodyIndex :type Integer) (bFromSweep :type Boolean) (SweepResult :type Hit%20Result%20Structure%20%28by%20ref%29))
  (Utilities|FlowControl|Sequence
    (:then_0
      (bind _asprojetil_do_heroi (Utilities|Casting|CastToProjetilDoHeroi OtherActor))
      (Variables|Default|SetHP (- (Variables|Default|GetHP) (Variables|Default|GetDano%20do%20Rifle)))
      (Actor|DestroyActor _asprojetil_do_heroi)
      (Variables|Default|SetRecebeu%20Dano true :!label _label)
      (if (<= (Variables|Default|GetHP) 0.0)
        (CallFunction|MorteDoAlien)))
    (:then_1
      (bind _asprojetil_do_heroi_2 (Utilities|Casting|CastToProjetilDoHeroi_2 OtherActor))
      (Variables|Default|SetHP (- (Variables|Default|GetHP) (Variables|Default|GetDano%20laser)))
      (Actor|DestroyActor _asprojetil_do_heroi_2)
      (goto _label))
    (:then_2
      (Audio|PlaySound2D "/Game/SFX/Alien_Atingido.Alien_Atingido" 1.1))))

(event Custom|Chegando%20na%20fazenda
  ;[0.3175 1 0.8186] Animaçao na fazenda
  (if (Variables|Default|GetParaTudo)
    (Components|Animation|PlayAnimation (Variables|Character|GetMesh) "/Game/Animações/Alien_01_Waving.Alien_01_Waving" true)))

(event Custom|Atacar
  (params (Character :type Jogador%20Object%20Reference))
  ;[1 1 1] Atacar
  (if (not (Variables|Default|GetParaTudo))
    (if (Variables|Default|GetSeen)
      (if (Variables|Default|GetClose%20Enough)
        (Audio|Components|Audio|Play (Variables|Default|GetTiro_Alien) 0.0)
        (Game|SpawnActorfromClass "/Game/BluePrints/ProjetilAlien.ProjetilAlien_C" (Transformation|GetWorldTransform (Variables|Default|GetGun)) "Undefined" 0 0)))))

(event Custom|Morte%20do%20Alien
  (bind _mesh (Variables|Character|GetMesh))
  (bind _returnvalue (Transformation|GetRelativeTransform _mesh))
  (Audio|Components|Audio|Play (Variables|Default|GetAlien_Morte) 0.0)
  (Variables|/Game/BluePrints/Jogador.Jogador_C|SetCaveiras (Variables|Default|GetJogador) (+ (Variables|/Game/BluePrints/Jogador.Jogador_C|GetCaveiras (Variables|Default|GetJogador)) 1.0))
  (Pawn|Components|CharacterMovement|DisableMovement (Variables|Character|GetCharacterMovement))
  (Collision|SetActorEnableCollision self false)
  (Components|Animation|PlayAnimation (Variables|Character|GetMesh) "/Game/Animações/Alien_01_Death.Alien_01_Death" false)
  (Utilities|FlowControl|Delay 3.0)
  (Components|MoveComponentTo _mesh (Math|Vector|MakeVector (.x (.location _returnvalue)) (.y (.location _returnvalue)) -1e+02) (.rotation _returnvalue) true true 1.0 false)
  (Game|SpawnActorfromClass "/Game/BluePrints/LazerGun_Item.LazerGun_Item_C" (Transformation|GetWorldTransform (Variables|Collision|GetCapsuleComponent)) "Undefined" 0 0)
  (Actor|DestroyActor))

(event EventBeginPlay)

(event EventTick
  (params (DeltaSeconds :type Float%20%28single-precision%29))
  (bind _capsulecomponent (Variables|Collision|GetCapsuleComponent))
  (bind _returnvalue (Class|PrimitiveComponent|IsOverlappingComponent _capsulecomponent))
  ;[1 0.9876 0.439] Ir para Fazenda
  (if (not (Variables|Default|GetSeen))
    (AI|AIMoveTo self "33.000000,-4231.000000, 0" 0 5.0 _returnvalue
      (:then
        (bind _output_get (Variables|Default|SetNa%20Fazenda _returnvalue))
        (if _output_get
          (Components|Animation|PlayAnimation (Variables|Character|GetMesh) "/Game/Animações/Alien_01_Waving.Alien_01_Waving" false :!label _label)
          (if (AI|Components|NavMovement|IsMovingonGround (Variables|Character|GetCharacterMovement))
            (Components|Animation|SetAnimationMode (Variables|Character|GetMesh) "AnimationBlueprint")
            (if (<= (Variables|Default|GetHP) 0.0)
              (CallFunction|MorteDoAlien)))))
      (:OnSuccess
        (goto _label)))))

(fn ConstructionScript)