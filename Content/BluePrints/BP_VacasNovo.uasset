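; Cow actor that the player can pick up before a UFO abducts it.
; A delayed random roll on Tick triggers Abduzir, which lowers three ship legs, plays beam audio, lifts Mech and reduces the player's VACOMETRO.
; Player overlap with Box instead calls PegarVaca and sets TemVaca, if no cow is already carried.
; Both paths call LevantarPernas to raise the legs and destroy the actor.
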(event OnComponentBeginOverlap(Box)
  (params (OverlappedComponent :type Primitive%20Component%20Object%20Reference) (OtherActor :type Actor%20Object%20Reference) (OtherComp :type Primitive%20Component%20Object%20Reference) (OtherBodyIndex :type Integer) (bFromSweep :type Boolean) (SweepResult :type Hit%20Result%20Structure%20%28by%20ref%29))
  (bind _mech (Variables|Default|GetMech))
  ;[1 1 1] Tocando na vaca
  (if (== OtherActor (Game|Player|GetPlayerPawn 0))
    (Variables|Default|SetTocando true)
    (bind _asjogador (Utilities|Casting|CastToJogador (Game|GetPlayerCharacter 0)))
    (if (not (Variables|/Game/BluePrints/Jogador.Jogador_C|GetTem%20Vaca _asjogador))
      (Default|PegarVaca _asjogador)
      (Rendering|ToggleVisibility _mech false)
      (Collision|SetCollisionEnabled _mech "NoCollision")
      (Variables|/Game/BluePrints/Jogador.Jogador_C|SetTem%20Vaca _asjogador true)
      (CallFunction|LevantarPernas))))

(event OnComponentEndOverlap(Box)
  (params (OverlappedComponent :type Primitive%20Component%20Object%20Reference) (OtherActor :type Actor%20Object%20Reference) (OtherComp :type Primitive%20Component%20Object%20Reference) (OtherBodyIndex :type Integer))
  ;[1 1 1] Tocando na vaca
  (if (== OtherActor (Game|Player|GetPlayerPawn 0))
    (Variables|Default|SetTocando false)))

(event Custom|Abduzir
  (bind _perna_1 (Variables|Default|GetPerna%201))
  (bind _perna_2 (Variables|Default|GetPerna%202))
  (bind _perna_3 (Variables|Default|GetPerna%203))
  (bind _mech (Variables|Default|GetMech))
  (bind _returnvalue (Transformation|GetRelativeTransform _perna_1))
  (bind _returnvalue_2 (Transformation|GetRelativeTransform _perna_2))
  (bind _returnvalue_3 (Transformation|GetRelativeTransform _perna_3))
  ;[1 1 1] ABDUÇÂO DA VACA
  (Collision|SetCollisionEnabled (Variables|Collision|GetCapsuleComponent) "NoCollision")
  (Pawn|Components|CharacterMovement|DisableMovement (Variables|Character|GetCharacterMovement))
  (Variables|Default|SetbUseControllerRotationYaw false)
  (Rendering|ToggleVisibility (Variables|Default|GetSpotlight) false)
  (Rendering|ToggleVisibility (Variables|Default|GetPerna%203) false)
  (Audio|Components|Audio|Play (Variables|Default|Getfeixe01) 0.0)
  (Audio|Components|Audio|Play (Variables|Default|GetVaca) 0.0)
  (Utilities|FlowControl|Delay 1.0)
  (Audio|Components|Audio|Play (Variables|Default|Getfeixeloop) 0.0)
  (Components|MoveComponentTo _perna_1 (Math|Vector|MakeVector (.x (.location _returnvalue)) (.y (.location _returnvalue)) 0.0) (.rotation _returnvalue) true false 0.5 false)
  (Audio|Components|Audio|Play (Variables|Default|GetPernasDescendoAudio) 0.0)
  (Components|MoveComponentTo _perna_2 (Math|Vector|MakeVector (.x (.location _returnvalue_2)) (.y (.location _returnvalue_2)) 0.1) (.rotation _returnvalue_2) true false 0.5 false)
  (Audio|Components|Audio|Play (Variables|Default|GetPernasDescendoAudio) 0.0)
  (Components|MoveComponentTo _perna_3 (Math|Vector|MakeVector (.x (.location _returnvalue_3)) (.y (.location _returnvalue_3)) 0.1) (.rotation _returnvalue_3) true false 0.5 false)
  (Audio|Components|Audio|Play (Variables|Default|GetPernasDescendoAudio) 0.0)
  (Collision|SetCollisionEnabled _mech "NoCollision")
  (Components|MoveComponentTo _mech "0.000000, 0,500.000000" "0, 0, 0" true false 1e+01 false)
  (CallFunction|LevantarPernas)
  (Audio|Components|Audio|Stop (Variables|Default|Getfeixeloop))
  (Audio|Components|Audio|Play (Variables|Default|Getfeixefim) 0.0)
  (Rendering|SetVisibility (Variables|Default|GetMech) false false)
  (bind _asjogador (Utilities|Casting|CastToJogador (Game|GetPlayerCharacter 0)))
  (Variables|/Game/BluePrints/Jogador.Jogador_C|SetVACOMETRO _asjogador (- (Variables|/Game/BluePrints/Jogador.Jogador_C|GetVACOMETRO _asjogador) 1e+01))
  (Utilities|FlowControl|Delay 2.0)
  (Actor|DestroyActor))

(event Custom|Levantar%20Pernas
  (bind _perna_1 (Variables|Default|GetPerna%201))
  (bind _perna_2 (Variables|Default|GetPerna%202))
  (bind _perna_3 (Variables|Default|GetPerna%203))
  (bind _returnvalue (Transformation|GetRelativeTransform _perna_3))
  (bind _returnvalue_2 (Transformation|GetRelativeTransform _perna_1))
  (bind _returnvalue_3 (Transformation|GetRelativeTransform _perna_2))
  ;[1 1 1] Levantando as pernas da nave e destruindo o BP
  (Rendering|ToggleVisibility (Variables|Default|GetConedeluz) false)
  (Components|MoveComponentTo _perna_1 (Math|Vector|MakeVector (.x (.location _returnvalue_2)) (.y (.location _returnvalue_2)) 1e+03) (.rotation _returnvalue_2) false true (Variables|Default|GetTempo%20de%20animação%20da%20perna) false)
  (Components|MoveComponentTo _perna_2 (Math|Vector|MakeVector (.x (.location _returnvalue_3)) (.y (.location _returnvalue_3)) 1e+03) (.rotation _returnvalue_3) false true (Variables|Default|GetTempo%20de%20animação%20da%20perna) false)
  (Components|MoveComponentTo _perna_3 (Math|Vector|MakeVector (.x (.location _returnvalue)) (.y (.location _returnvalue)) 1e+03) (.rotation _returnvalue) false true (Variables|Default|GetTempo%20de%20animação%20da%20perna) false)
  (Audio|Components|Audio|Stop (Variables|Default|Getfeixeloop))
  (Utilities|FlowControl|Delay 1.0)
  (Actor|DestroyActor))

(event EventTick
  (params (DeltaSeconds :type Float%20%28single-precision%29))
  ;[1 1 1] Tempo randomico para bduções
  (Utilities|FlowControl|Delay (Variables|Default|GetDelay%20da%20Abducao))
  (switch int (Math|Random|RandomIntegerinRange 0 10)
    (:0
      (CallFunction|Abduzir))))

(fn ConstructionScript)