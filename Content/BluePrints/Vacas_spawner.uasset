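; Cow (Vacas) spawner actor that keeps populating the level with AI-driven BP_VacasNovo pawns up to a maximum count.
; BeginPlay starts a looping SpawnVacas timer at a per-second rate, targeting the first Vacas_spawner found in the world rather than itself.
; Each tick of that timer counts existing cows and, below the cap, spawns one with Vacas_BehaviorTree at a random point inside SpawnVolume.
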(event Custom|SpawnVacas
  (bind _spawnvolume (Variables|Default|GetSpawnVolume))
  (bind _outactors (Actor|GetAllActorsOfClass "/Game/BluePrints/BP_VacasNovo.BP_VacasNovo_C"))
  (if (< (Utilities|Array|Length _outactors) (Variables|Default|GetMaximo%20de%20vacas))
    (AI|SpawnAIFromClass "/Game/BluePrints/BP_VacasNovo.BP_VacasNovo_C" "/Game/BehaviourTree/Vacas_BehaviorTree.Vacas_BehaviorTree" (Math|Random|RandomPointinBoundingBox (Transformation|GetWorldLocation _spawnvolume) (Components|Box|GetScaledBoxExtent _spawnvolume)) "0, 0, 0" false)))

(event EventBeginPlay
  (bind _outactors (Actor|GetAllActorsOfClass "Vacas_spawner_C"))
  (bind _output_get (Variables|Default|SetSpawner (Utilities|Array|Get(acopy) _outactors)))
  (Utilities|Time|SetTimerbyFunctionName _output_get "SpawnVacas" (/ 1.0 (Variables|Default|GetVacas%20por%20segundo)) true))

(fn ConstructionScript)